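; BP_AsitoAI is a Totori character with simple ambient AI that alternates randomly between idling and wandering.
; The first Tick starts a looping timer that calls CycleAction every few seconds, beginning immediately.
; CycleAction either stops movement and turns toward a random TotoriLookTarget-tagged actor, or walks to a random reachable point nearby.
; Each branch plays its looping animation directly on the mesh.
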(event `self.ReceiveTick`
  (params (DeltaSeconds :type "Float (single-precision)"))
  (`/Engine/EditorBlueprintResources/StandardMacros.DoOnce` false
    (:`Completed`
      (`KismetSystemLibrary.K2_SetTimer` null "CycleAction" 4.5 true false 1.0)
      (`self.CycleAction`))))

(fn `CycleAction`
  (bind _returnvalue (`self.GetController`))
  (bind _returnvalue_2 (`self.K2_GetActorLocation`))
  (bind _mesh (`self.Mesh`))
  (if (`KismetMathLibrary.RandomBool`)
    (bind _outactors (`GameplayStatics.GetAllActorsWithTag` "TotoriLookTarget"))
    (`AIBlueprintHelperLibrary.SimpleMoveToLocation` _returnvalue _returnvalue_2)
    (`self.K2_SetActorRotation` (`KismetMathLibrary.FindLookAtRotation` _returnvalue_2 (`self.K2_GetActorLocation` (`KismetArrayLibrary.Array_Random` _outactors))))
    (`SkeletalMeshComponent.PlayAnimation` _mesh "/Game/Totoris/Anim/Totori_idle_neutral_Anim.Totori_idle_neutral_Anim" true)
    (else
      (`SkeletalMeshComponent.PlayAnimation` _mesh "/Game/Totoris/Anim/Totori_walk_forward.Totori_walk_forward" true)
      (`AIBlueprintHelperLibrary.SimpleMoveToLocation` _returnvalue (`NavigationSystemV1.K2_GetRandomReachablePointInRadius` (`self.K2_GetActorLocation`) 550.0 null null)))))

(fn `ReceiveBeginPlay_0`)

(fn `UserConstructionScript`)